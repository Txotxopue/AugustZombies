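; BP_ArrozPickup is an ammo pickup that floats, spins and grants ammo to overlapping actors implementing BPI_AmmoPicker.
; After a random start delay, the FloatingAnimation timeline applies PlayRate-scaled vertical offsets to the mesh, clamping its relative height.
; Tick yaws the mesh at SpinSpeed.
; The trigger sphere overlap uses DoOnce to send AmmoAmountInPickup through the interface once, then destroys the pickup.
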(event `self.ReceiveBeginPlay`
  (bind (_relativelocation_x _relativelocation_y _relativelocation_z) (`KismetMathLibrary.BreakVector` (`SceneComponent.RelativeLocation` (`self.PickupMesh`))))
  (`TimelineComponent.SetPlayRate` (`self.FloatingAnimation`) (`self.PlayRate`))
  (`KismetSystemLibrary.Delay` (`KismetMathLibrary.RandomFloatInRange` 0.0 5.0))
  (bind (_direction _vectorlerpalpha) (`Timeline|FloatingAnimation`)
    (:`Update`
      (`SceneComponent.K2_AddLocalOffset` (`self.PickupMesh`) (* (`KismetMathLibrary.MakeVector` 0.0 0.0 _vectorlerpalpha) (`self.PlayRate`)) false)
      (if (> _relativelocation_z 50.0)
        (`SceneComponent.K2_SetRelativeLocation` (`self.PickupMesh`) (0.0 0.0 50.0) false)
        (elif (< _relativelocation_z -50.0)
          (`SceneComponent.K2_SetRelativeLocation` (`self.PickupMesh`) (0.0 0.0 -50.0) false))))))

(event `self.ReceiveActorBeginOverlap`
  (params (OtherActor :type "Actor Object Reference")))

(event `self.ReceiveTick`
  (params (DeltaSeconds :type "Float (single-precision)"))
  (`SceneComponent.K2_AddLocalRotation` (`self.PickupMesh`) (`KismetMathLibrary.MakeRotator` 0.0 (* DeltaSeconds (`self.SpinSpeed`))) false))

(event `self.TriggerSphere.OnComponentBeginOverlap`
  (params (OtherActor :type "Actor Object Reference") (OtherComp :type "PrimitiveComponent Object Reference") (OtherBodyIndex :type Integer) (bFromSweep :type Boolean) (SweepResult :type "HitResult Structure (by ref)"))
  (if (`KismetSystemLibrary.DoesImplementInterface` OtherActor "/Game/Blueprints/Interfaces/BPI_AmmoPicker.BPI_AmmoPicker_C")
    (`/Engine/EditorBlueprintResources/StandardMacros.DoOnce` false
      (:`Completed`
        (message `/Game/Blueprints/Interfaces/BPI_AmmoPicker.PickupAmmo` OtherActor (`self.AmmoAmountInPickup`))
        (`self.K2_DestroyActor`)))))

(fn `UserConstructionScript`)