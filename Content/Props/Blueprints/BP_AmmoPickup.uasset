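; Ammo pickup prop that floats and spins until an actor able to pick up ammo walks into it.
; A timeline, started after a random delay, bobs the mesh up and down, while Tick rotates it by a spin speed.
; Trigger sphere overlap checks for the BPI_AmmoPicker interface, sends the ammo amount through an interface message once, then destroys the pickup.
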(event `self.ReceiveBeginPlay`
  (`KismetSystemLibrary.Delay` (`KismetMathLibrary.RandomFloatInRange` 0.0 5.0))
  (bind (_direction _vectorlerpalpha) (`Timeline|FloatingAnimation`)
    (:`Update`
      (`SceneComponent.K2_AddWorldOffset` (`self.PickupMesh`) (* (`KismetMathLibrary.VLerp` (0.0 0.0 10.0) (0.0 0.0 -10.0) _vectorlerpalpha) (`GameplayStatics.GetWorldDeltaSeconds`)) false))))

(event `self.ReceiveActorBeginOverlap`
  (params (OtherActor :type "Actor Object Reference")))

(event `self.ReceiveTick`
  (params (DeltaSeconds :type "Float (single-precision)"))
  (`SceneComponent.K2_AddLocalRotation` (`self.PickupMesh`) (`KismetMathLibrary.MakeRotator` 0.0 (* DeltaSeconds (`self.SpinSpeed`))) false))

(event `self.TriggerSphere.OnComponentBeginOverlap`
  (params (OtherActor :type "Actor Object Reference") (OtherComp :type "PrimitiveComponent Object Reference") (OtherBodyIndex :type Integer) (bFromSweep :type Boolean) (SweepResult :type "HitResult Structure (by ref)"))
  (if (`KismetSystemLibrary.DoesImplementInterface` OtherActor "/Game/Blueprints/Interfaces/BPI_AmmoPicker.BPI_AmmoPicker_C")
    (`/Engine/EditorBlueprintResources/StandardMacros.DoOnce` false
      (:`Completed`
        (message `/Game/Blueprints/Interfaces/BPI_AmmoPicker.PickupAmmo` OtherActor (`self.AmmoAmountInPickup`))
        (`self.K2_DestroyActor`)))))

(fn `UserConstructionScript`)