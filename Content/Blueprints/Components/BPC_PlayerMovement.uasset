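; Actor component that provides basic movement, look and jump functions for the player's Character.
; On BeginPlay it caches its owner as a Character, and each function forwards calls or axis values to that owner.
; Rate-based look functions scale input by base rates and frame time, while Turn and LookUp pass it raw.
; Jump also plays a sound at the character's location when CanJump is true.
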(event `self.ReceiveTick`
  (params (DeltaSeconds :type "Float (single-precision)")))

(event `self.ReceiveBeginPlay`
  (bind _ascharacter (cast `Character` (`self.GetOwner`)))
  (set `self.OwnerActor` _ascharacter))

(fn `Jump`
  (`Character.Jump` (`self.OwnerActor`))
  (if (`Character.CanJump` (`self.OwnerActor`))
    (`GameplayStatics.PlaySoundAtLocation` "/Game/Audio/SFX/SC_Jump_Cue.SC_Jump_Cue" (`Actor.K2_GetActorLocation` (`self.OwnerActor`)))))

(fn `LookUp`
  (params (InputAxisValue :type "Float (double-precision)"))
  (`Pawn.AddControllerPitchInput` (`self.OwnerActor`) InputAxisValue))

(fn `LookUpRate`
  (params (InputAxisValue :type "Float (double-precision)"))
  (`Pawn.AddControllerPitchInput` (`self.OwnerActor`) (* InputAxisValue (`self.BaseLookUpRate`) (`GameplayStatics.GetWorldDeltaSeconds`))))

(fn `MoveForward`
  (params (InputAxisValue :type "Float (double-precision)"))
  (bind _owneractor (`self.OwnerActor`))
  (`Pawn.AddMovementInput` _owneractor (`Actor.GetActorForwardVector` _owneractor) InputAxisValue false))

(fn `MoveRight`
  (params (InputAxisValue :type "Float (double-precision)"))
  (bind _owneractor (`self.OwnerActor`))
  (`Pawn.AddMovementInput` _owneractor (`Actor.GetActorRightVector` _owneractor) InputAxisValue false))

(fn `StopJumping`
  (`Character.StopJumping` (`self.OwnerActor`)))

(fn `Turn`
  (params (InputAxisValue :type "Float (double-precision)"))
  (`Pawn.AddControllerYawInput` (`self.OwnerActor`) InputAxisValue))

(fn `TurnRate`
  (params (InputAxisValue :type "Float (double-precision)"))
  (`Pawn.AddControllerYawInput` (`self.OwnerActor`) (* InputAxisValue (`self.BaseTurnRate`) (`GameplayStatics.GetWorldDeltaSeconds`))))