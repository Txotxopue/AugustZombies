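; Weapon component for BP_PlayerCharacter that handles hitscan firing, ammo use and capped ammo pickups.
; FireWeapon checks ammo, plays the montage and spends ammo immediately, while sound and a camera-forward trace from screen center follow ShotDelay.
; Hits spawn particles and apply point or radial damage by weapon type, so even grenade explosions are traced.
; Projectile spawning and beam tracer helpers exist but never run; the tracer is marked unfinished.
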(event `self.ReceiveTick`
  (params (DeltaSeconds :type "Float (single-precision)")))

(event `self.ReceiveBeginPlay`
  (bind _asbp_player_character (cast `/Game/Blueprints/BP_PlayerCharacter` (`self.GetOwner`)))
  (set `self.OwnerActor` _asbp_player_character))

(event `Fire Weapon`
  (params (WeaponFired :type "/Game/___TEST_Zombies/ENUM_WeaponTypes Enum"))
  (bind _hasammo (`self.CheckAmmo`))
  (if _hasammo
    (`|ExecutionSequence`
      (:`then_0`
        (`self.PlayDefaultAnimation`))
      (:`then_1`
        (`KismetSystemLibrary.Delay` (`self.ShotDelay`))
        (`self.PlayShotSFX`)
        (bind (_hashit _outhit) (`self.CheckRaytraceHit`))
        (if _hashit
          (`self.InstanceHitParticles` _outhit WeaponFired)
          (`self.DoDamage` _outhit WeaponFired)))
      (:`then_2`
        (`self.UseAmmo` (`self.UsedAmmoAmountPerShot`))))))

(event `/Game/Blueprints/Interfaces/BPI_AmmoPicker.PickupAmmo`
  (params (AmmoAmount :type Integer))
  (bind _maxammo (`self.MaxAmmo`))
  (bind _returnvalue (+ AmmoAmount (`self.CurrentAmmo`)))
  (if (> _returnvalue _maxammo)
    (set `self.CurrentAmmo` _maxammo)
    (else
      (set `self.CurrentAmmo` _returnvalue))))

(fn `BulletTraceFX`
  (bind _returnvalue (`self.K2_GetComponentLocation`))
  (bind _returnvalue_2 (`GameplayStatics.SpawnEmitterAtLocation` "/Game/Effects/Particles/PS_BulletTrace.PS_BulletTrace" _returnvalue))
  (`ParticleSystemComponent.SetBeamTargetPoint` _returnvalue_2 0 (`self.LastHitLocation`) 0)
  (`ParticleSystemComponent.SetBeamSourcePoint` _returnvalue_2 0 _returnvalue 0)
  (return))

(fn `CheckAmmo`
  (returns (HasAmmo :type Boolean))
  (bind _returnvalue (> (`self.CurrentAmmo`) 0))
  (if (not _returnvalue)
    (`GameplayStatics.PlaySoundAtLocation` "/Game/Audio/SFX/SW_OutOfAmmo.SW_OutOfAmmo" (`self.K2_GetComponentLocation`)))
  (return _returnvalue))

(fn `CheckRaytraceHit`
  (returns (HasHit :type Boolean) (OutHit :type "HitResult Structure"))
  (bind _asbp_hud (cast `/Game/Blueprints/BP_HUD` (`PlayerController.GetHUD` (`GameplayStatics.GetPlayerController` 0)))
    (:`then`
      (bind _screencentercoordinates (`/Game/Blueprints/BP_HUD.GetScreenCenter` _asbp_hud))
      (bind _worldlocation (`PlayerController.DeprojectScreenPositionToWorld` (`GameplayStatics.GetPlayerController` 0) (`KismetMathLibrary.BreakVector2D` _screencentercoordinates) (`.Y` (`KismetMathLibrary.BreakVector2D` _screencentercoordinates))))
      (bind (_outhit _returnvalue) (`KismetSystemLibrary.LineTraceSingle` :`Start` _worldlocation :`End` (+ _worldlocation (* (`KismetMathLibrary.GetForwardVector` (`self.K2_GetComponentRotation` (`/Game/Blueprints/BP_PlayerCharacter.FirstPersonCamera` (`self.OwnerActor`)))) (`self.GunRange`))) :`TraceChannel` "TraceTypeQuery3" :`DrawDebugType` "ForDuration")))
    (:`CastFailed`
      _))
  (return _returnvalue _outhit))

(fn `DoDamage`
  (params (Hit :type "HitResult Structure") (WeaponFired :type "/Game/___TEST_Zombies/ENUM_WeaponTypes Enum"))
  (if (`|EnumEquality` WeaponFired "NewEnumerator0")
    (`GameplayStatics.ApplyDamage` Hit_HitActor (`self.WeaponDamage`))
    (elif (`|EnumEquality` WeaponFired "NewEnumerator1")
      (`GameplayStatics.ApplyRadialDamage` (`self.GrenadeDamage`) Hit_Location (`self.GrenadeRadius`)))))

(fn `InstanceHitParticles`
  (params (Hit :type "HitResult Structure") (WeaponFired :type "/Game/___TEST_Zombies/ENUM_WeaponTypes Enum"))
  (bind (_bblockinghit _binitialoverlap _time _location _impactpoint _normal) (`GameplayStatics.BreakHitResult` Hit))
  (bind _returnvalue (`KismetMathLibrary.Conv_VectorToRotator` _normal))
  (set `self.LastHitLocation` _location)
  (if (`|EnumEquality` WeaponFired "NewEnumerator0")
    (`GameplayStatics.SpawnEmitterAtLocation` "/Game/Effects/Particles/PS_HitDefault.PS_HitDefault" _location _returnvalue)
    (elif (`|EnumEquality` WeaponFired "NewEnumerator1")
      (`GameplayStatics.SpawnEmitterAtLocation` "/Game/Effects/Particles/PS_Explosion_Bomb.PS_Explosion_Bomb" _location _returnvalue))))

(fn `PlayDefaultAnimation`
  (`AnimInstance.Montage_Play` (`SkeletalMeshComponent.GetAnimInstance` (`/Game/Blueprints/BP_PlayerCharacter.Mesh2P` (`self.OwnerActor`))) "/Game/FirstPersonBP/Animations/FirstPerson_Fire_Montage.FirstPerson_Fire_Montage" 1.0)
  (return))

(fn `PlayShotSFX`
  (`GameplayStatics.PlaySoundAtLocation` "/Game/FirstPersonBP/Audio/FirstPerson_WeaponFire.FirstPerson_WeaponFire" (`self.K2_GetComponentLocation`))
  (return))

(fn `SpawnDefaultProjectile`
  (`|SpawnActorFromClass` "/Game/FirstPersonBP/Blueprints/FirstPersonProjectile.FirstPersonProjectile_C" (`KismetMathLibrary.MakeTransform` (`self.K2_GetComponentLocation`) (`Pawn.GetControlRotation` (`self.OwnerActor`))))
  (return))

(fn `UseAmmo`
  (params (UsedAmmoAmount :type Integer))
  (bind _returnvalue (- (`self.CurrentAmmo`) UsedAmmoAmount))
  (if (< _returnvalue 0)
    (set `self.CurrentAmmo` 0)
    (else
      (set `self.CurrentAmmo` _returnvalue)))
  (return))