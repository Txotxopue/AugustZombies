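; BP_ZombiPlaceholder is a placeholder zombie actor that wanders procedurally, without AI or navigation.
; BeginPlay uses a random stream to set a starting yaw and a time offset.
; Tick feeds offset game time into a clamped tangent for stop-and-go movement along local Y, and into a sine for a slowly swaying yaw.
; Both steps are applied per frame without delta-time scaling, so speed depends on frame rate.
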(event `self.ReceiveBeginPlay`
  (bind _returnvalue (* (`KismetMathLibrary.RandomFloatFromStream` (`self.Random Stream Seed`)) 100.0))
  (`self.SetActorRotation` (`KismetMathLibrary.MakeRotator` 0.0 _returnvalue))
  (set `self.Random Number` _returnvalue))

(event `self.ReceiveActorBeginOverlap`
  (params (OtherActor :type "Actor Object Reference")))

(event `self.ReceiveTick`
  (params (DeltaSeconds :type "Float (single-precision)"))
  (`self.K2_AddActorLocalOffset` (`KismetMathLibrary.MakeVector` 0.0 (* (`KismetMathLibrary.FClamp` (`KismetMathLibrary.Tan` (/ (+ (`KismetSystemLibrary.GetGameTimeInSeconds`) (`self.Random Number`)) 10.0))) 0.1)))
  (`self.K2_AddActorLocalRotation` (`KismetMathLibrary.MakeRotator` 0.0 (* (`KismetMathLibrary.Sin` (* (+ (`KismetSystemLibrary.GetGameTimeInSeconds`) (`self.Random Number`)) 0.1)) 0.5))))

(fn `UserConstructionScript`)